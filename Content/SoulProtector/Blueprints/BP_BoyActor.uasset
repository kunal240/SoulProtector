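; BP_BoyActor is an actor that floats upward, then disappears in a burst of dust.
; Each Tick it moves up by a fixed, frame-rate-dependent step with a swept SetActorLocation.
; Above a world height threshold it attaches P_Dust emitters to its Mesh every tick and destroys itself after a short Delay.
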(event `self.ReceiveTick`
  (params (DeltaSeconds :type "Float (single-precision)"))
  (bind (_returnvalue_x _returnvalue_y _returnvalue_z) (`KismetMathLibrary.BreakVector` (`self.K2_GetActorLocation`)))
  (bind _returnvalue (+ _returnvalue_z 3.0))
  (`/Engine/EditorBlueprintResources/StandardMacros.IsValid` (`ActorComponent.GetOwner` (`self.DefaultSceneRoot`))
    (:`Is Valid`
      (`self.K2_SetActorLocation` (`KismetMathLibrary.MakeVector` _returnvalue_x _returnvalue_y _returnvalue) true)
      (if (> _returnvalue 3000.0)
        (`GameplayStatics.SpawnEmitterAttached` "/Game/SoulProtector/ParticleSystems/Dust/P_Dust.P_Dust" (`self.Mesh`) "None" (0.0 0.0 0.0) (struct) (1.0 1.0 1.0) "SnapToTargetIncludingScale")
        (`KismetSystemLibrary.Delay` 2.0)
        (`self.K2_DestroyActor`)))))

(fn `UserConstructionScript`)