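; BP_Minion is an enemy that takes melee damage from BP_Hermes and plays directional hit reactions.
; On capsule overlap, chained checks test punch state, hand or elbow collider, and dot-product angle to choose a back, front, left or right montage, then call CheckHealth.
; MeleeDamage, capped at remaining Health, is also subtracted in fall-through branches, so non-punch overlaps cause damage and some hits subtract it twice.
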(event `self.ReceiveBeginPlay`)

(event `self.ReceiveTick`
  (params (DeltaSeconds :type "Float (single-precision)")))

(event `self.CapsuleComponent.OnComponentBeginOverlap`
  (params (OverlappedComponent :type "PrimitiveComponent Object Reference") (OtherActor :type "Actor Object Reference") (OtherComp :type "PrimitiveComponent Object Reference") (OtherBodyIndex :type Integer) (bFromSweep :type Boolean) (SweepResult :type "HitResult Structure (by ref)"))
  (bind _health (`self.Health`))
  (bind _asbp_hermes (cast `/Game/SoulProtector/Blueprints/BP_Hermes` OtherActor))
  (bind _returnvalue (and (`/Game/SoulProtector/Blueprints/BP_Hermes.IsPunching?` _asbp_hermes) (or (== OtherComp (`/Game/SoulProtector/Blueprints/BP_Hermes.RightHandCollision` _asbp_hermes)) (== OtherComp (`/Game/SoulProtector/Blueprints/BP_Hermes.LeftHandCollision` _asbp_hermes)) (== OtherComp (`/Game/SoulProtector/Blueprints/BP_Hermes.RightElbowCollision` _asbp_hermes)))))
  (bind _returnvalue_2 (`KismetMathLibrary.DegAcos` (`KismetMathLibrary.Dot_VectorVector` (* (`SceneComponent.GetForwardVector` (`self.CapsuleComponent`)) (-1.0 0.0 0.0)) (`self.GetActorForwardVector` _asbp_hermes))))
  (if (and _returnvalue (`KismetMathLibrary.InRange_FloatFloat` _returnvalue_2 120.0 180.0))
    (bind _returnvalue_3 (- _health (`KismetMathLibrary.FMin` _health (`Hermes.MeleeDamage` _asbp_hermes))))
    (set `self.Health` _returnvalue_3)
    (`|PlayMontage` (`self.Mesh`) "/Game/SoulProtector/Animation/MinionAnimations/AM_GotHitBack.AM_GotHitBack"
      (:`then`
        (`self.CheckHealth`)))
    (else
      (set `self.Health` _returnvalue_3)
      (if (and _returnvalue (`KismetMathLibrary.InRange_FloatFloat` _returnvalue_2 0.0 60.0))
        (`|PlayMontage` (`self.Mesh`) "/Game/SoulProtector/Animation/MinionAnimations/AM_GotHitFront.AM_GotHitFront"
          (:`then`
            (`self.CheckHealth`)))
        (else
          (bind _returnvalue_4 (`KismetMathLibrary.DegAcos` (`KismetMathLibrary.Dot_VectorVector` (`SceneComponent.GetRightVector` (`self.CapsuleComponent`)) (`self.GetActorForwardVector` _asbp_hermes))))
          (if (and _returnvalue (`KismetMathLibrary.InRange_FloatFloat` _returnvalue_4 150.0 180.0))
            (set `self.Health` _returnvalue_3)
            (`|PlayMontage` (`self.Mesh`) "/Game/SoulProtector/Animation/MinionAnimations/AM_GotHitLeft.AM_GotHitLeft"
              (:`then`
                (`self.CheckHealth`)))
            (else
              (set `self.Health` _returnvalue_3)
              (if (and _returnvalue (`KismetMathLibrary.InRange_FloatFloat` _returnvalue_4 0.0 30.0))
                (`|PlayMontage` (`self.Mesh`) "/Game/SoulProtector/Animation/MinionAnimations/AM_GotHitRight.AM_GotHitRight"
                  (:`then`
                    (`self.CheckHealth`)))))))))))

(fn `UserConstructionScript`)